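; BP_Gold is a gold trigger actor that notifies other objects through interface messages when something overlaps its Box.
; Each overlap sends AlexBallCollitionActionINter to Bpcubo, then branches on PlayerGold to choose Aaaperro's message.
; Aaaperro receives AlexBallCollition2 while the flag is false and AlexBallCollitionActionINter once it is true; both branches set PlayerGold true.
; BeginPlay runs a GetActorOfClass lookup with no visible use of its result.
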(event OnComponentBeginOverlap(Box)
  (params (OverlappedComponent :type Primitive%20Component%20Object%20Reference) (OtherActor :type Actor%20Object%20Reference) (OtherComp :type Primitive%20Component%20Object%20Reference) (OtherBodyIndex :type Integer) (bFromSweep :type Boolean) (SweepResult :type Hit%20Result%20Structure%20%28by%20ref%29))
  (bind _aaaperro (Variables|Default|Getaaaperro))
  (Class|AlexInterfaces|AlexBallCollitionActionINter(Message) (Variables|Default|Getbpcubo))
  (if (Variables|Default|GetplayerGold)
    (Class|AlexInterfaces|AlexBallCollitionActionINter(Message) _aaaperro)
    (Variables|Default|SetplayerGold true)
    (else
      (Class|AlexInterfaces|AlexBallCollition2(Message) _aaaperro)
      (Variables|Default|SetplayerGold true))))

(event EventBeginPlay
  (Actor|GetActorOfClass 0))

(event Collision|EventActorBeginOverlap
  (params (OtherActor :type Actor%20Object%20Reference)))

(event EventTick
  (params (DeltaSeconds :type Float%20%28single-precision%29)))

(fn ConstructionScript)